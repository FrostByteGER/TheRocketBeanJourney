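; AI controller Blueprint that moves its controlled pawn to a target supplied through the AddnewtargetPosition event.
; The event waits briefly, then issues an AI MoveTo toward the supplied Position, used as the target actor, with an acceptance radius.
; Debug prints trace the request, its result and the success or fail outcome; BeginPlay, Tick and the construction script are empty.
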(event `Add new target Position`
  (params (position :type "Actor Object Reference"))
  (`KismetSystemLibrary.PrintString` "Hello 123")
  (`KismetSystemLibrary.Delay` 2.0)
  (bind _movementresult (`|AIMoveTo` (`self.K2_GetPawn`) (0.0 0.0 0.0) position 150.0)
    (:`then`
      (`KismetSystemLibrary.PrintString` "Hello 1234")
      (switch `EPathFollowingResult` _movementresult
        (:`Success`
          (`KismetSystemLibrary.PrintString` "Path Success"))
        (:`Blocked`
          (`KismetSystemLibrary.PrintString` "Path Blocked"))
        (:`OffPath`
          (`KismetSystemLibrary.PrintString` "Path Off"))
        (:`Aborted`
          (`KismetSystemLibrary.PrintString` "aborted"))
        (:`Skipped`
          (`KismetSystemLibrary.PrintString` "Path Skipped"))
        (:`Invalid`
          (`KismetSystemLibrary.PrintString` "invalid"))))
    (:`OnSuccess`
      (`KismetSystemLibrary.PrintString` "Success"))
    (:`OnFail`
      (`KismetSystemLibrary.PrintString` "Fail"))))

(event `self.ReceiveBeginPlay`)

(event `self.ReceiveTick`
  (params (DeltaSeconds :type "Float (single-precision)")))

(fn `UserConstructionScript`)