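; Paper2D character pawn driven by player input despite its AI name, restarting the level when destroyed.
; Move axes add world-space movement and call UpdateAnimation, which derives an eight-way LastDirection from velocity to pick walk or idle flipbooks and rotate DirectionArrow.
; Interact line-traces along that arrow and calls OnInteract on any hit BP_Interactible.
; Holding Transform only sets and prints a Transformed flag.
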(event `InputAction|Interact`
  (params (Key :type "Key Structure" :default "AnyKey"))
  (bind _returnvalue (`self.K2_GetActorLocation`))
  (:`Pressed`
    (`KismetSystemLibrary.PrintString` "INTERACT")
    (bind (_outhit _returnvalue_2) (`KismetSystemLibrary.LineTraceSingle` :`Start` _returnvalue :`End` (+ _returnvalue (* (`KismetMathLibrary.GetForwardVector` (`SceneComponent.K2_GetComponentRotation` (`self.DirectionArrow`))) (`self.InteractionDistance`))) :`TraceChannel` "TraceTypeQuery3" :`DrawDebugType` "ForDuration"))
    (if _returnvalue_2
      (bind _asbp_interactible (cast `/Game/HitNut/Blueprints/BP_Interactible` (`.HitActor` (`GameplayStatics.BreakHitResult` _outhit))))
      (`/Game/HitNut/Blueprints/BP_Interactible.OnInteract` _asbp_interactible self))))

(event `OnPlayerDeath`
  ;[1 1 1] Restart Level on Death
  (`KismetSystemLibrary.ExecuteConsoleCommand` "RestartLevel"))

(event `self.ReceiveBeginPlay`
  ;[1 1 1] Restart Level on Death
  (add `self.OnDestroyed` (delegate `OnPlayerDeath`)))

(event `InputAction|Transform`
  (params (Key :type "Key Structure" :default "AnyKey"))
  (:`Pressed`
    (if (not (`self.Transformed`))
      (bind _output_get (set `self.Transformed` true))
      (`KismetSystemLibrary.PrintString` (`KismetStringLibrary.Conv_BoolToString` _output_get))))
  (:`Released`
    (if (`self.Transformed`)
      (bind _output_get_2 (set `self.Transformed` false))
      (`KismetSystemLibrary.PrintString` (`KismetStringLibrary.Conv_BoolToString` _output_get_2)))))

(event `UpdateAnimation`
  (bind (_returnvalue_x _returnvalue_y) (`KismetMathLibrary.BreakVector` (`self.GetVelocity`)))
  (bind _returnvalue (`MovementComponent.GetMaxSpeed` (`self.CharacterMovement`)))
  (bind _returnvalue_2 (/ _returnvalue_y _returnvalue))
  (bind _returnvalue_3 (- (/ _returnvalue_x _returnvalue) 0.0))
  ;[1 1 1] MovementBlending
  (if (and (> _returnvalue_2 0.0) (== _returnvalue_3 0.0))
    (set `self.LastDirection` "NewEnumerator2")
    (`PaperFlipbookComponent.SetFlipbook` (`self.Sprite`) (select `/Game/HitNut/Blueprints/Direction` (`self.LastDirection`) :`NewEnumerator0` "/Game/HitNut/Sprites/Character/Walk/FP_Walk_Back.FP_Walk_Back" :`NewEnumerator1` "/Game/HitNut/Sprites/Character/Walk/FP_Walk_Side_Back_Right.FP_Walk_Side_Back_Right" :`NewEnumerator2` "/Game/HitNut/Sprites/Character/Walk/FP_Walk_Side_Front_Right.FP_Walk_Side_Front_Right" :`NewEnumerator3` "/Game/HitNut/Sprites/Character/Walk/FP_Walk_Side_Front_Right.FP_Walk_Side_Front_Right" :`NewEnumerator4` "/Game/HitNut/Sprites/Character/Walk/FP_Walk_Front.FP_Walk_Front" :`NewEnumerator5` "/Game/HitNut/Sprites/Character/Walk/FP_Walk_Side_Front_Left.FP_Walk_Side_Front_Left" :`NewEnumerator6` "/Game/HitNut/Sprites/Character/Walk/FP_Walk_Side_Front_Left.FP_Walk_Side_Front_Left" :`NewEnumerator7` "/Game/HitNut/Sprites/Character/Walk/FP_Walk_Side_Back_Left.FP_Walk_Side_Back_Left" :!type "PaperFlipbook Object Reference") :!label _label)
    (elif (and (< _returnvalue_2 0.0) (== _returnvalue_3 0.0))
      (set `self.LastDirection` "NewEnumerator6")
      (goto _label)
      (elif (and (== _returnvalue_2 0.0) (> _returnvalue_3 0.0))
        (set `self.LastDirection` "NewEnumerator0")
        (goto _label)
        (elif (and (== _returnvalue_2 0.0) (< _returnvalue_3 0.0))
          (set `self.LastDirection` "NewEnumerator4")
          (goto _label)
          (elif (and (> _returnvalue_2 0.0) (> _returnvalue_3 0.0))
            (set `self.LastDirection` "NewEnumerator1")
            (goto _label)
            (elif (and (< _returnvalue_2 0.0) (> _returnvalue_3 0.0))
              (set `self.LastDirection` "NewEnumerator7")
              (goto _label)
              (elif (and (> _returnvalue_2 0.0) (< _returnvalue_3 0.0))
                (set `self.LastDirection` "NewEnumerator3")
                (goto _label)
                (elif (and (< _returnvalue_2 0.0) (< _returnvalue_3 0.0))
                  (set `self.LastDirection` "NewEnumerator5")
                  (goto _label)
                  (else
                    (`PaperFlipbookComponent.SetFlipbook` (`self.Sprite`) (select `/Game/HitNut/Blueprints/Direction` (`self.LastDirection`) :`NewEnumerator0` "/Game/HitNut/Sprites/Character/Idle/FP_Idle_Back.FP_Idle_Back" :`NewEnumerator1` "/Game/HitNut/Sprites/Character/Idle/FP_Idle_Side_Back_Right.FP_Idle_Side_Back_Right" :`NewEnumerator2` "/Game/HitNut/Sprites/Character/Idle/FP_Idle_Side_Front_Right.FP_Idle_Side_Front_Right" :`NewEnumerator3` "/Game/HitNut/Sprites/Character/Idle/FP_Idle_Side_Front_Right.FP_Idle_Side_Front_Right" :`NewEnumerator4` "/Game/HitNut/Sprites/Character/Idle/FP_Idle_Front.FP_Idle_Front" :`NewEnumerator5` "/Game/HitNut/Sprites/Character/Idle/FP_Idle_Side_Front_Left.FP_Idle_Side_Front_Left" :`NewEnumerator6` "/Game/HitNut/Sprites/Character/Idle/FP_Idle_Side_Front_Left.FP_Idle_Side_Front_Left" :`NewEnumerator7` "/Game/HitNut/Sprites/Character/Idle/FP_Idle_Side_Back_Left.FP_Idle_Side_Back_Left" :!type "PaperFlipbook Object Reference")))))))))))
  (`SceneComponent.K2_SetRelativeRotation` (`self.DirectionArrow`) (`KismetMathLibrary.MakeRotator` 0.0 0.0 (select `/Game/HitNut/Blueprints/Direction` (`self.LastDirection`) :`NewEnumerator1` 45.0 :`NewEnumerator2` 90.0 :`NewEnumerator3` 135.0 :`NewEnumerator4` 180.0 :`NewEnumerator5` 225.0 :`NewEnumerator6` 270.0 :`NewEnumerator7` 315.0 :!type "Float (single-precision)")) false false))

(event `InputAxis|MoveRight`
  (params (AxisValue :type "Float (single-precision)"))
  ;[1 1 1] Left/Right Movement
  (`self.AddMovementInput` (0.0 1.0 0.0) AxisValue)
  (`self.UpdateAnimation`))

(event `InputAxis|MoveUp`
  (params (AxisValue :type "Float (single-precision)"))
  ;[1 1 1] Up/Down Movement
  (`self.AddMovementInput` (1.0 0.0 0.0) AxisValue)
  (`self.UpdateAnimation`))

(fn `UserConstructionScript`)