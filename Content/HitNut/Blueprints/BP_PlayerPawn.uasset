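; Player pawn with a Paper2D flipbook sprite that moves on two world axes and restarts the level when destroyed.
; Axis inputs add movement and refresh the flipbook; left/right flips the sprite, while up/down sets control rotation to zero.
; The flipbook select lists eight idle/walk variants, but its boolean X-velocity index only reaches the side-front pair.
; BeginPlay binds destruction to a RestartLevel console command.
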(event `OnPlayerDeath`
  ;[1 1 1] Restart Level on Death
  (`KismetSystemLibrary.ExecuteConsoleCommand` "RestartLevel"))

(event `self.ReceiveBeginPlay`
  ;[1 1 1] Restart Level on Death
  (add `self.OnDestroyed` (delegate `OnPlayerDeath`)))

(event `UpdateAnimation`
  (bind (_returnvalue_x _returnvalue_y) (`KismetMathLibrary.BreakVector` (`self.GetVelocity`)))
  (`PaperFlipbookComponent.SetFlipbook` (`self.Sprite`) (select `int` (`KismetMathLibrary.Conv_BoolToInt` (> (`KismetMathLibrary.Abs` (/ _returnvalue_x (`MovementComponent.GetMaxSpeed` (`self.CharacterMovement`)))) 0.0)) :`0` "/Game/HitNut/Sprites/Character/Idle/Idle_Side_Front.Idle_Side_Front" :`1` "/Game/HitNut/Sprites/Character/Walk/Walk_Side_Front.Walk_Side_Front" :`2` "/Game/HitNut/Sprites/Character/Idle/Idle_Side_Back.Idle_Side_Back" :`3` "/Game/HitNut/Sprites/Character/Walk/Walk_Side_Back.Walk_Side_Back" :`4` "/Game/HitNut/Sprites/Character/Idle/Idle_Front.Idle_Front" :`5` "/Game/HitNut/Sprites/Character/Walk/Walk_Front.Walk_Front" :`6` "/Game/HitNut/Sprites/Character/Idle/Idle_Back.Idle_Back" :`7` "/Game/HitNut/Sprites/Character/Walk/Walk_Back.Walk_Back" :!type "PaperFlipbook Object Reference")))

(event `InputAxis|MoveRight`
  (params (AxisValue :type "Float (single-precision)"))
  (bind _sprite (`self.Sprite`))
  ;[1 1 1] Left/Right Movement
  (`self.AddMovementInput` (0.0 1.0 0.0) AxisValue)
  (`self.UpdateAnimation`)
  (`/Engine/EditorBlueprintResources/StandardMacros.CompareFloat` AxisValue
    (:`>`
      (`SceneComponent.K2_SetRelativeRotation` _sprite (`KismetMathLibrary.MakeRotator` 90.0 180.0 -90.0) false false))
    (:`<`
      (`SceneComponent.K2_SetRelativeRotation` _sprite (`KismetMathLibrary.MakeRotator` 90.0 0.0 -90.0) false false))))

(event `InputAxis|MoveUp`
  (params (AxisValue :type "Float (single-precision)"))
  ;[1 1 1] Up/Down Movement
  (`self.AddMovementInput` (1.0 0.0 0.0) AxisValue)
  (`self.UpdateAnimation`)
  (`/Engine/EditorBlueprintResources/StandardMacros.CompareFloat` AxisValue
    (:`>`
      (`Controller.SetControlRotation` (`self.GetController`) (`KismetMathLibrary.MakeRotator` 0.0)))
    (:`<`
      (`Controller.SetControlRotation` (`self.GetController`) (`KismetMathLibrary.MakeRotator` 0.0 0.0 0.0)))))

(fn `UserConstructionScript`)