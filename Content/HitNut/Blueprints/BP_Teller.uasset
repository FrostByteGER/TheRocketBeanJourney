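; BP_Teller is an interactable that players can bait with a specific nut to kill AI-controlled pawns.
; When a non-AI pawn interacts, it checks the first inventory item against NutName, then either consumes it and sets NutPlaced or prints a wrong-nut message.
; When a pawn driven by BP_AI_Controller interacts, CheckInteractConditions returns NutPlaced, and if true that pawn is killed.
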(event `/Game/HitNut/Blueprints/BPI_Interactible.OnInteract`
  (params (Instigator :type "Actor Object Reference"))
  (bind _asbp_player_pawn (cast `/Game/HitNut/Blueprints/BP_PlayerPawn` Instigator))
  (bind _asbp_ai_controller (cast `/Game/HitNut/Blueprints/BP_AI_Controller` (`Pawn.GetController` _asbp_player_pawn))
    (:`then`
      (bind _caninteract_ (`self.CheckInteractConditions` _asbp_ai_controller))
      (if _caninteract_
        (bind _asbp_player_pawn_2 (cast `/Game/HitNut/Blueprints/BP_PlayerPawn` (`Controller.K2_GetPawn` _asbp_ai_controller)))
        (`/Game/HitNut/Blueprints/BP_PlayerPawn.Kill` _asbp_player_pawn_2)))
    (:`CastFailed`
      (if (not (`self.NutPlaced`))
        (bind _inventory (`/Game/HitNut/Blueprints/BP_PlayerPawn.Inventory` _asbp_player_pawn))
        (if (== (`/Game/HitNut/Blueprints/BP_Pickup.Name` (`KismetArrayLibrary.Array_Get` _inventory)) (`self.NutName`))
          (set `self.NutPlaced` true)
          (`KismetArrayLibrary.Array_Remove` _inventory)
          (`KismetSystemLibrary.PrintString` "PLACED NUT")
          (else
            (`KismetSystemLibrary.PrintString` "Wrong Nut!")))))))

(fn `CheckInteractConditions`
  (params (Actor :type "Actor Object Reference"))
  (returns (`CanInteract?` :type Boolean))
  (return (`self.NutPlaced`)))

(fn `UserConstructionScript`
  (`parent.UserConstructionScript`))